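; AIC_Runner is an AI controller that drives a BP_Runner pawn by simulating alternating left and right power inputs.
; On possession it caches the runner, and on BeginPlay it starts a timer with a random delay between minimum and maximum input delays.
; Each SimulateInput event flip-flops between left and right, then schedules the next timer with a new random delay, producing irregular input pacing.
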(event `self.ReceiveBeginPlay`
  (`KismetSystemLibrary.K2_SetTimerDelegate` (`|CreateDelegate` :!event `SimulateInput`) (`KismetMathLibrary.RandomFloatInRange` (`self.MinInputDelay`) (`self.MaxInputDelay`)) :!label _label))

(event `self.ReceivePossess`
  (params (PossessedPawn :type "Pawn Object Reference"))
  (bind _asbp_runner (cast `/Game/Blueprints/BP_Runner` PossessedPawn))
  (set `self.Owning Runner` _asbp_runner))

(event `SimulateInput`
  (`/Engine/EditorBlueprintResources/StandardMacros.FlipFlop`
    (:`A`
      (`/Game/Blueprints/BP_Runner.SimulatePowerLeft` (`self.Owning Runner`))
      (goto _label))
    (:`B`
      (`/Game/Blueprints/BP_Runner.SimpulatePowerRight` (`self.Owning Runner`))
      (goto _label))))

(fn `UserConstructionScript`)